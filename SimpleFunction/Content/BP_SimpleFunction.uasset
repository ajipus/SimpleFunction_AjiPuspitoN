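; BP_SimpleFunction is a small Blueprint that exercises simple functions, with results printed to screen.
; On BeginPlay a loop repeatedly calls PointPlayer, which adds Hit to Score, printing each running total and then "Finish".
; AttackPlayer subtracts Damage from HealthPoint and returns it, as does the identical, uncalled AttackPlayerImp.
; The Boolean branch and health test in the event graph are disconnected and never run.
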(event EventBeginPlay
  ;[1 1 1] SimpleFunctionScore
  (for _index (range 0 10)
    (Development|PrintString (Utilities|String|ToString(Integer) (CallFunction|PointPlayer (Variables|Default|GetHit))) true true "(R=0.000000,G=0.660000,B=1.000000,A=1.000000)" 15.0))
  (Development|PrintString "Finish" true true "(R=0.000000,G=0.660000,B=1.000000,A=1.000000)" 2e+01))

(fn ConstructionScript)

(fn AttackPlayer
  (params (Damage :type Integer))
  (bind _output_get (Variables|Default|SetHealthPoint (- (Variables|Default|GetHealthPoint) Damage)))
  (return _output_get))

(fn AttackPlayerImp
  (params (Damage :type Integer))
  (bind _output_get (Variables|Default|SetHealthPoint (- (Variables|Default|GetHealthPoint) Damage)))
  (return _output_get))

(fn PointPlayer
  (params (Hit :type Integer))
  (bind _output_get (Variables|Default|SetScore (+ (Variables|Default|GetScore) Hit)))
  (return _output_get))